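; Player character Blueprint that handles movement, door interaction and attacking.
; MoveX and MoveY feed movement input along world-space diagonals, rotating the controls 45 degrees from the world axes.
; BeginPlay loops over all DoorBP actors but keeps only the last, which Interact destroys if its CanOpen is true.
; Attack spawns AttackBP at a fixed world-space offset from the character, regardless of facing.
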(event EventBeginPlay
  (Variables|Default|SetOverlap false)
  (Variables|Default|SetButtonPress false)
  (bind _outactors (Actor|GetAllActorsOfClass "/Game/DoorBP.DoorBP_C"))
  (for _array_element _outactors
    (Variables|Default|SetDoorRef _array_element)))

(event Input|ActionEvents|InputActionInteract
  (params (Key :type Key%20Structure))
  (:Pressed
    (if (Variables|/Game/DoorBP.DoorBP_C|GetcanOpen (Variables|Default|GetDoorRef))
      (Actor|DestroyActor (Variables|Default|GetDoorRef)))))

(event Input|ActionEvents|InputActionAttack
  (params (Key :type Key%20Structure))
  (:Pressed
    (Game|SpawnActorfromClass "/Game/AttackBP.AttackBP_C" (Math|Conversions|ToTransform(Vector) (+ (Transformation|GetActorLocation) "100.000000,0.000000,100.000000")) "Undefined" 0 0)))

(event Input|AxisEvents|InputAxisMoveX
  (params (AxisValue :type Float%20%28single-precision%29))
  (Pawn|Input|AddMovementInput (Math|Vector|Normalize (Math|Vector|MakeVector 1.0 -1.0 0.0)) AxisValue false))

(event Input|AxisEvents|InputAxisMoveY
  (params (AxisValue :type Float%20%28single-precision%29))
  (Pawn|Input|AddMovementInput (Math|Vector|Normalize (Math|Vector|MakeVector 1.0 1.0 0.0)) AxisValue false))

(fn ConstructionScript)